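; TextCheckpoint_BP is a text display that changes its message when a checkpoint is flagged as reached.
; The construction script fills the TextRender with Test, and BeginPlay switches it to Text1 after a short delay.
; Tick and the delayed BeginPlay chain share a CheckpointReached check that sets Text2 when true, polled every frame.
; Nothing in this graph sets CheckpointReached.
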(event `self.ReceiveBeginPlay`
  (bind _textrender (`self.TextRender`))
  (`KismetSystemLibrary.Delay` 2.5)
  (`TextRenderComponent.K2_SetText` _textrender (`self.text1`))
  (if (`self.checkpointReached?`) :!label _label
    (`TextRenderComponent.K2_SetText` _textrender (`self.text2`))))

(event `self.ReceiveTick`
  (params (DeltaSeconds :type "Float (single-precision)"))
  (goto _label))

(fn `UserConstructionScript`
  (`TextRenderComponent.K2_SetText` (`self.TextRender`) (`self.test`)))