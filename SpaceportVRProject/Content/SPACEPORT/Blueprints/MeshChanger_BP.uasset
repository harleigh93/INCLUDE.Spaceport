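; MeshChanger_BP is a VR prop that a BP_MotionController can pick up and that changes into an iPad mesh on contact.
; Pickup turns off physics and attaches the actor to the supplied component, while Drop detaches it and restores physics.
; When a motion controller overlaps the sphere collision, ChangeMesh swaps the static mesh to IPad, with debug prints tracing the steps.
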(event `self.ReceiveBeginPlay`)

(event `/Game/VirtualRealityBP/Blueprints/PickupActorInterface.Pickup`
  (params (AttachTo :type "SceneComponent Object Reference"))
  (`PrimitiveComponent.SetSimulatePhysics` (`self.StaticMeshComponent`) false)
  (`SceneComponent.K2_AttachToComponent` (`self.K2_GetRootComponent`) AttachTo "None" "KeepWorld" "KeepWorld" "KeepWorld" false))

(event `/Game/VirtualRealityBP/Blueprints/PickupActorInterface.Drop`
  (`PrimitiveComponent.SetSimulatePhysics` (`self.StaticMeshComponent`) true)
  (`self.K2_DetachFromActor` "KeepWorld" "KeepWorld" "KeepWorld"))

(event `Key|Y`
  (params (Key :type "Key Structure")))

(event `ChangeMesh`
  (`KismetSystemLibrary.PrintString` "In Custom Event")
  (`StaticMeshComponent.SetStaticMesh` (`self.StaticMeshComponent`) "/Game/SPACEPORT/Meshes/HUB_Assets/iPad.iPad")
  (`KismetSystemLibrary.PrintString` "Leaving Function"))

(event `self.SphereColl.OnComponentBeginOverlap`
  (params (OverlappedComponent :type "PrimitiveComponent Object Reference") (OtherActor :type "Actor Object Reference") (OtherComp :type "PrimitiveComponent Object Reference") (OtherBodyIndex :type Integer) (bFromSweep :type Boolean) (SweepResult :type "HitResult Structure (by ref)"))
  (cast `/Game/VirtualRealityBP/Blueprints/BP_MotionController` OtherActor)
  (`KismetSystemLibrary.PrintString` "5 Pressed")
  (`self.ChangeMesh`)
  (`KismetSystemLibrary.PrintString` "Changed Mesh"))

(fn `UserConstructionScript`)