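; Syringe prop for the plant level that motion controllers can grab to water lettuce plant pillows.
; Pickup turns off physics and attaches it to the given component; Drop re-enables physics and detaches it.
; Its SyringeColl overlap fills it from a water bag, then spends that water on a pillow that has dirt but no water.
; A successful watering marks the pillow watered and instantly reveals its full-grown lettuce mesh.
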(event `/Game/VirtualRealityBP/Blueprints/PickupActorInterface.Pickup`
  (params (AttachTo :type "SceneComponent Object Reference"))
  (`PrimitiveComponent.SetSimulatePhysics` (`self.StaticMeshComponent`) false)
  (`SceneComponent.K2_AttachToComponent` (`self.K2_GetRootComponent`) AttachTo "None" "KeepWorld" "KeepWorld" "KeepWorld" false))

(event `/Game/VirtualRealityBP/Blueprints/PickupActorInterface.Drop`
  (`PrimitiveComponent.SetSimulatePhysics` (`self.StaticMeshComponent`) true)
  (`self.K2_DetachFromActor` "KeepWorld" "KeepWorld" "KeepWorld"))

(event `self.SyringeColl.OnComponentBeginOverlap`
  (params (OverlappedComponent :type "PrimitiveComponent Object Reference") (OtherActor :type "Actor Object Reference") (OtherComp :type "PrimitiveComponent Object Reference") (OtherBodyIndex :type Integer) (bFromSweep :type Boolean) (SweepResult :type "HitResult Structure (by ref)"))
  (cast `/Game/SPACEPORT/Blueprints/PlantLevel_BPs/plantWaterBag_BP` OtherActor
    (:`then`
      (set `self.haswater?` true))
    (:`CastFailed`
      (bind _asplant_pillow_bp (cast `/Game/SPACEPORT/Blueprints/PlantLevel_BPs/plantPillow_BP` OtherActor))
      (if (`/Game/SPACEPORT/Blueprints/PlantLevel_BPs/plantPillow_BP.dirtdirt?` _asplant_pillow_bp)
        (if (`self.haswater?`)
          (if (not (`/Game/SPACEPORT/Blueprints/PlantLevel_BPs/plantPillow_BP.water?` _asplant_pillow_bp))
            (set `/Game/SPACEPORT/Blueprints/PlantLevel_BPs/plantPillow_BP.water?` true _asplant_pillow_bp)
            (`SceneComponent.SetVisibility` (`/Game/SPACEPORT/Blueprints/PlantLevel_BPs/plantPillow_BP.lettuceFullGrown` _asplant_pillow_bp) true false)
            (set `self.haswater?` false)))))))

(fn `UserConstructionScript`)