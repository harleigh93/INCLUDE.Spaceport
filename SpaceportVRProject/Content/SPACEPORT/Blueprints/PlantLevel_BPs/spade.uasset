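; Grabbable spade for the plant level that carries dirt from a bag to a plant pillow.
; Pickup, called by the motion controller, disables physics and attaches it; Drop detaches it and re-enables physics.
; Sphere overlap with bagOfDirt shows the dirt component and sets Dirt.
; Overlapping plantPillow_BP while Dirt is set flags that pillow as dirt-filled and hides the dirt, but never clears Dirt.
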(event `/Game/VirtualRealityBP/Blueprints/PickupActorInterface.Pickup`
  (params (AttachTo :type "SceneComponent Object Reference"))
  (`PrimitiveComponent.SetSimulatePhysics` (`self.StaticMeshComponent`) false)
  (`SceneComponent.K2_AttachToComponent` (`self.K2_GetRootComponent`) AttachTo "None" "KeepWorld" "KeepWorld" "KeepWorld" false))

(event `/Game/VirtualRealityBP/Blueprints/PickupActorInterface.Drop`
  (`PrimitiveComponent.SetSimulatePhysics` (`self.StaticMeshComponent`) true)
  (`self.K2_DetachFromActor` "KeepWorld" "KeepWorld" "KeepWorld"))

(event `self.Sphere.OnComponentBeginOverlap`
  (params (OverlappedComponent :type "PrimitiveComponent Object Reference") (OtherActor :type "Actor Object Reference") (OtherComp :type "PrimitiveComponent Object Reference") (OtherBodyIndex :type Integer) (bFromSweep :type Boolean) (SweepResult :type "HitResult Structure (by ref)"))
  (cast `/Game/SPACEPORT/Blueprints/PlantLevel_BPs/bagOfDirt` OtherActor
    (:`then`
      (`SceneComponent.SetVisibility` (`self.dirtdirtdirt`) true false)
      (set `self.dirt?` true))
    (:`CastFailed`
      (`KismetSystemLibrary.PrintString` "Not dirt")
      (bind _asplant_pillow_bp (cast `/Game/SPACEPORT/Blueprints/PlantLevel_BPs/plantPillow_BP` OtherActor))
      (if (`self.dirt?`)
        (set `/Game/SPACEPORT/Blueprints/PlantLevel_BPs/plantPillow_BP.dirtdirt?` true _asplant_pillow_bp)
        (`SceneComponent.SetVisibility` (`self.dirtdirtdirt`) false false)
        (else
          (`KismetSystemLibrary.PrintString` "no dirt"))))))

(fn `UserConstructionScript`)