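; LookingText_BP is a world-space text actor that shows two timed messages once the welcome text has spawned.
; Each Tick, until it has fired, it polls the SpawnedWelcomeText flag on SpaceportGameInstance.
; When the flag is true it latches Spawned, sets its TextRender to Text1, then switches to Text2 after a short delay.
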(event `self.ReceiveBeginPlay`)

(event `self.ReceiveTick`
  (params (DeltaSeconds :type "Float (single-precision)"))
  (if (not (`self.Spawned?`))
    (bind _asspaceport_game_instance (cast `/Game/SPACEPORT/SpaceportGameInstance` (`GameplayStatics.GetGameInstance`)))
    (if (`/Game/SPACEPORT/SpaceportGameInstance.SpawnedWelcomeText?` _asspaceport_game_instance)
      (set `self.Spawned?` true)
      (`TextRenderComponent.K2_SetText` (`self.TextRender`) (`self.Text1`))
      (`KismetSystemLibrary.Delay` 3.5)
      (`TextRenderComponent.K2_SetText` (`self.TextRender`) (`self.Text2`)))))

(fn `UserConstructionScript`)