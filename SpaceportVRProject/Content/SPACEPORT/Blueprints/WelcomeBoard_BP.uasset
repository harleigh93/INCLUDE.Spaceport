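; WelcomeBoard_BP is the spaceport's welcome billboard, showing intro text to the player.
; On BeginPlay it registers itself, its collision and its intro text with SpaceportGameInstance.
; Tick polls the game instance's SpawnedWelcomeText flag and, once it is set, runs a one-shot sequence guarded by Spawned.
; That sequence swaps the intro text for a second title and steps through three text parts on timed delays.
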(event `self.ReceiveBeginPlay`
  (bind _asspaceport_game_instance (cast `/Game/SPACEPORT/SpaceportGameInstance` (`GameplayStatics.GetGameInstance`))
    (:`then`
      (set `/Game/SPACEPORT/SpaceportGameInstance.WelcomeBillboard` (`self.BillboardCollision`) _asspaceport_game_instance)
      (set `/Game/SPACEPORT/SpaceportGameInstance.WelcomeTextRef` (`self.SpaceportIntroText`) _asspaceport_game_instance)
      (set `/Game/SPACEPORT/SpaceportGameInstance.WelcomeBoardRef` self _asspaceport_game_instance))
    (:`CastFailed`
      (`KismetSystemLibrary.PrintString` "WRONG CAST"))))

(event `self.ReceiveTick`
  (params (DeltaSeconds :type "Float (single-precision)"))
  (if (not (`self.Spawned?`))
    (bind _asspaceport_game_instance (cast `/Game/SPACEPORT/SpaceportGameInstance` (`GameplayStatics.GetGameInstance`)))
    (if (`/Game/SPACEPORT/SpaceportGameInstance.SpawnedWelcomeText?` _asspaceport_game_instance)
      (`SceneComponent.SetVisibility` (`self.SpaceportIntroText`) false false)
      (set `self.Spawned?` true)
      (`SceneComponent.SetVisibility` (`self.Intro2Title`) true false)
      (`SceneComponent.SetVisibility` (`self.Intro2Part1`) true false)
      (`KismetSystemLibrary.Delay` 6.0)
      (`SceneComponent.SetVisibility` (`self.Intro2Part1`) false false)
      (`SceneComponent.SetVisibility` (`self.Intro2Part2`) true false)
      (`KismetSystemLibrary.Delay` 5.0)
      (`SceneComponent.SetVisibility` (`self.Intro2Part2`) false false)
      (`SceneComponent.SetVisibility` (`self.Intro2Part3`) true false))))

(fn `UserConstructionScript`)