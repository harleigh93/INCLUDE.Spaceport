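; Text render actor in the Spaceport content that shows a timed sequence of messages.
; The construction script sets the TextRender component to the Test variable as its initial text.
; BeginPlay then uses chained delays to swap in Text1 and later Text2, once each with no loop.
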(event `self.ReceiveBeginPlay`
  (bind _textrender (`self.TextRender`))
  (`KismetSystemLibrary.Delay` 8.0)
  (`TextRenderComponent.K2_SetText` _textrender (`self.text1`))
  (`KismetSystemLibrary.Delay` 4.0)
  (`TextRenderComponent.K2_SetText` _textrender (`self.text2`)))

(fn `UserConstructionScript`
  (`TextRenderComponent.K2_SetText` (`self.TextRender`) (`self.test`)))